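; BP_FlamePillar is an actor that makes its FireLight flicker like a flame by varying the light's intensity.
; A looping timer started at BeginPlay picks a new target as a random percentage step from the current intensity, clamped between a fraction of the base and a fixed maximum.
; Tick eases the current intensity toward that target with FInterpTo and applies it to the light, smoothing the random walk.
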(event Custom|Flicker
  (Variables|Default|SetTargetIntensity (Math|Float|Clamp(Float) (* (Variables|Default|GetCurrentIntensity) (+ (Math|Random|RandomFloatinRange (- 0.0 (Variables|Default|GetMaxChangePercent)) (+ 0.0 (Variables|Default|GetMaxChangePercent))) 1.0)) (* (Variables|Default|GetBaseIntensity) 0.6) 5e+03)))

(event EventBeginPlay
  (bind _baseintensity (Variables|Default|GetBaseIntensity))
  (Variables|Default|SetCurrentIntensity _baseintensity)
  (Variables|Default|SetTargetIntensity _baseintensity)
  (bind _returnvalue (Utilities|Time|SetTimerbyEvent (delegate Custom|Flicker) 0.2 true))
  (Variables|Default|SetFlickerTimer _returnvalue)
  (Actor|Tick|SetActorTickEnabled true))

(event EventTick
  (params (DeltaSeconds :type Float%20%28single-precision%29))
  (bind _output_get (Variables|Default|SetCurrentIntensity (Math|Interpolation|FInterpTo (Variables|Default|GetCurrentIntensity) (Variables|Default|GetTargetIntensity) (Utilities|Time|GetWorldDeltaSeconds) (Variables|Default|GetInterpSpeed))))
  (Rendering|Components|Light|SetIntensity (Variables|Default|GetFireLight) _output_get))

(fn ConstructionScript)