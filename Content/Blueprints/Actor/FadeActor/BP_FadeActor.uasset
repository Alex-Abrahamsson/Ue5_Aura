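; BP_FadeActor is a mesh actor that can fade out and back in when its FadeOut and Fadein events are called.
; The construction script caches original materials and builds dynamic instances from FadeMaterialInstanses, which FadeOut swaps onto the mesh.
; A timeline, reversed for fade-in, drives their "Fade" parameter.
; On finish, full Fade restores original materials, and optional BlockVisibility toggles the Visibility channel between Block and Ignore by fade level.
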(event EventBeginPlay)

(event EventFadeOut
  (CallFunction|SetMatierialtoDynamicInstance)
  (bind _fade (Timeline|FadeTimeLine Play)
    (:Update
      (for _array_element (Variables|Default|GetDynamicMaterialInstace)
        (Rendering|Material|SetScalarParameterValue _array_element "Fade" _fade :!class /Script/Engine.MaterialInstanceDynamic)))
    (:Finished
      (CallFunction|FadeFinished _fade))))

(event EventFadein
  (bind _fade (Timeline|FadeTimeLine Reverse)
    (:Update
      (for _array_element (Variables|Default|GetDynamicMaterialInstace)
        (Rendering|Material|SetScalarParameterValue _array_element "Fade" _fade :!class /Script/Engine.MaterialInstanceDynamic)))
    (:Finished
      (CallFunction|FadeFinished _fade))))

(fn ConstructionScript
  (Utilities|Array|Clear (Variables|Default|GetDynamicMaterialInstace))
  (Variables|Default|SetOriginalMaterials (Rendering|Material|GetMaterials (Variables|Default|GetMesh)))
  (for _array_element (Variables|Default|GetFadeMaterialInstanses)
    (bind _returnvalue (Rendering|Material|CreateDynamicMaterialInstance _array_element "None" "None" :!class /Script/Engine.KismetMaterialLibrary))
    (Utilities|Array|AddUnique (Variables|Default|GetDynamicMaterialInstace) _returnvalue)))

(fn SetMatierialtoDynamicInstance
  (for (_array_element _array_index) (Variables|Default|GetDynamicMaterialInstace)
    (Rendering|Material|SetMaterial (Variables|Default|GetMesh) _array_index _array_element)))

(fn ResetMaterials
  (for (_array_element _array_index) (Variables|Default|GetOriginalMaterials)
    (Rendering|Material|SetMaterial (Variables|Default|GetMesh) _array_index _array_element)))

(fn FadeFinished
  (params (Fade :type Float%20%28double-precision%29))
  (bind _mesh (Variables|Default|GetMesh))
  (if (>= Fade 1.0)
    (CallFunction|ResetMaterials)
    (if (Variables|Default|GetBlockVisibility)
      (Collision|SetCollisionResponsetoChannel _mesh "ECC_Visibility" "ECR_Block"))
    (elif (<= Fade 0.3)
      (if (Variables|Default|GetBlockVisibility)
        (Collision|SetCollisionResponsetoChannel _mesh "ECC_Visibility" "ECR_Ignore")))))